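; BP_SurvivorController is the AI controller for survivors, running the BT_Survivor behavior tree on possess.
; When AI perception updates, HasPlayerInArray checks the updated actors for the "Player" tag and, on a match, sets the IsSpotted blackboard key to true.
; It does not check whether the player was sensed or lost, and the node that would clear IsSpotted is unconnected, so the controller never resets the flag.
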(event OnPerceptionUpdated(AIPerception)
  (params (UpdatedActors :type Array%20of%20Actor%20Object%20References))
  (bind _result (CallFunction|HasPlayerinArray UpdatedActors))
  (if _result
    (AI|Components|Blackboard|SetValueasBool (Variables|Default|GetBlackboard) (Utilities|Name|MakeLiteralName "IsSpotted") true)))

(event EventBeginPlay)

(event EventTick
  (params (DeltaSeconds :type Float%20%28single-precision%29)))

(event EventPossess
  (params (PossessedPawn :type Pawn%20Object%20Reference))
  (AI|RunBehaviorTree "/Game/Blueprints/BT_Survivor.BT_Survivor"))

(fn ConstructionScript)

(fn HasPlayerinArray
  (params (Actors :type Array%20of%20Actor%20Object%20References))
  (LocalVariables|SetHasAny false)
  (bind _array_element (Utilities|Array|ForEachLoopwithBreak Actors :!label _label)
    (:LoopBody
      (if (Actor|ActorHasTag _array_element "Player")
        (LocalVariables|SetHasAny true)
        (goto _label Break)))
    (:Completed
      (return (LocalVariables|GetHasAny)))))